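; BP_ButtonDoor is an actor pairing a button with a door, both moved vertically by an overlap on its Sphere component.
; BeginPlay caches both start locations.
; Overlap begin plays a pickup sound and runs a timeline whose two tracks offset each part's world Z from that start.
; Overlap end reverses the timeline, returning both parts toward their start, and no check filters the overlapping actor.
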(event OnComponentBeginOverlap(Sphere)
  (params (OverlappedComponent :type Primitive%20Component%20Object%20Reference) (OtherActor :type Actor%20Object%20Reference) (OtherComp :type Primitive%20Component%20Object%20Reference) (OtherBodyIndex :type Integer) (bFromSweep :type Boolean) (SweepResult :type Hit%20Result%20Structure%20%28by%20ref%29))
  (bind _initialbuttonlocation (Variables|Default|GetInitialButtonLocation))
  (bind _initialdoorlocation (Variables|Default|GetInitialDoorLocation))
  (Audio|PlaySound2D "/Game/Retro_8Bit_Sounds/Collectables/Cues/retro_collect_pickup_item_08_Cue.retro_collect_pickup_item_08_Cue" 1.0 1.0 0.0 0 0)
  (bind (_direction _valuetrackdown _valuedoortrack) (Timeline|Timeline_0 Play)
    (:Update
      (Transformation|SetWorldLocation (Variables|Default|GetButton) (Math|Vector|MakeVector (.x _initialbuttonlocation) (.y _initialbuttonlocation) (+ _valuetrackdown (.z _initialbuttonlocation))) false false)
      (Transformation|SetWorldLocation (Variables|Default|Getdoor) (Math|Vector|MakeVector (.x _initialdoorlocation) (.y _initialdoorlocation) (+ _valuedoortrack (.z _initialdoorlocation))) false false))))

(event OnComponentEndOverlap(Sphere)
  (params (OverlappedComponent :type Primitive%20Component%20Object%20Reference) (OtherActor :type Actor%20Object%20Reference) (OtherComp :type Primitive%20Component%20Object%20Reference) (OtherBodyIndex :type Integer))
  (bind _initialbuttonlocation (Variables|Default|GetInitialButtonLocation))
  (bind _initialdoorlocation (Variables|Default|GetInitialDoorLocation))
  (bind (_direction _valuetrackdown _valuedoortrack) (Timeline|Timeline_0 Reverse)
    (:Update
      (Transformation|SetWorldLocation (Variables|Default|GetButton) (Math|Vector|MakeVector (.x _initialbuttonlocation) (.y _initialbuttonlocation) (+ _valuetrackdown (.z _initialbuttonlocation))) false false)
      (Transformation|SetWorldLocation (Variables|Default|Getdoor) (Math|Vector|MakeVector (.x _initialdoorlocation) (.y _initialdoorlocation) (+ _valuedoortrack (.z _initialdoorlocation))) false false))))

(event EventBeginPlay
  (Variables|Default|SetInitialButtonLocation (Transformation|GetWorldLocation (Variables|Default|GetButton)))
  (Variables|Default|SetInitialDoorLocation (Transformation|GetWorldLocation (Variables|Default|Getdoor))))

(fn ConstructionScript)