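; Booster is a bounce pad that launches the BP_Ball when it hits the pad's mesh.
; On hit it applies a mass-independent impulse along the mesh's up vector and plays a 2D retro bounce sound.
; The ScaleBooster timeline offsets the mesh's Z scale from its BeginPlay value, with a retriggerable delay on each update that later reverses the timeline.
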(event OnComponentHit(StaticMesh)
  (params (HitComponent :type Primitive%20Component%20Object%20Reference) (OtherActor :type Actor%20Object%20Reference) (OtherComp :type Primitive%20Component%20Object%20Reference) (NormalImpulse :type Vector :default "0, 0, 0") (Hit :type Hit%20Result%20Structure%20%28by%20ref%29))
  (bind _beginscale (Variables|Default|GetBeginScale))
  (bind _asbp_ball (Utilities|Casting|CastToBP_Ball OtherActor))
  (Physics|AddImpulse (Variables|/Game/Rolling/Character/BP_Ball.BP_Ball_C|GetStaticMesh _asbp_ball) (* (Math|Vector|GetUpVector (Variables|Default|GetStaticMesh)) (Variables|Default|GetImpulse)) "None" true)
  (Audio|PlaySound2D "/Game/Retro_8Bit_Sounds/Jumping/Wavs/retro_jump_bounce_12.retro_jump_bounce_12" 1.0 1.0 0.0 0 0)
  (bind _boost (Timeline|Scale%20Booster Play)
    (:Update
      (Transformation|SetWorldScale3D (Variables|Default|GetStaticMesh) (Math|Vector|MakeVector (.x _beginscale) (.y _beginscale) (.z (+ (Variables|Default|GetBeginScale) _boost))))
      (Utilities|FlowControl|RetriggerableDelay 0.25)
      (Timeline|Scale%20Booster Reverse))))

(event EventBeginPlay
  ;[1 1 1] Set BeginScale
  (Variables|Default|SetBeginScale (Transformation|GetWorldScale (Variables|Default|GetStaticMesh))))

(fn ConstructionScript)