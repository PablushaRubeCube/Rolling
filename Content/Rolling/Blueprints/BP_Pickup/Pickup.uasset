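; BP_Pickup is a collectible actor that grants health, score and goal progress to BP_Ball.
; Sphere overlap calls PickupFunction, which updates the ball and plays a sound and particle effect.
; When Pickupable is set, the mesh gives way to an animated WBP_PickupCoin widget showing its Points; otherwise it is destroyed immediately.
; Any overlapping actor, ball or not, triggers destruction after a short delay.
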(event OnComponentBeginOverlap(Sphere)
  (params (OverlappedComponent :type Primitive%20Component%20Object%20Reference) (OtherActor :type Actor%20Object%20Reference) (OtherComp :type Primitive%20Component%20Object%20Reference) (OtherBodyIndex :type Integer) (bFromSweep :type Boolean) (SweepResult :type Hit%20Result%20Structure%20%28by%20ref%29))
  (CallFunction|PickupFunction OtherActor)
  (Utilities|FlowControl|Delay 0.5)
  (Actor|DestroyActor))

(event EventBeginPlay
  ;[1 1 1] off visibility WBP_PickupCoin
  (Rendering|SetVisibility (Variables|Default|GetWidget) false false)
  ;;[1 1 1] Set Points for WBP_PickupCoin
  (bind _aswbp_pickup_coin (Utilities|Casting|CastToWBP_PickupCoin (UserInterface|GetUserWidgetObject (Variables|Default|GetWidget))))
  (Variables|/Game/Rolling/Blueprints/HUD/WBP_PickupCoin.WBP_PickupCoin_C|SetPickupValue _aswbp_pickup_coin (Variables|Default|GetPoints)))

(fn ConstructionScript)

(fn PickupFunction
  (params (Object :type Object%20Object%20Reference))
  (bind _asbp_ball (Utilities|Casting|CastToBP_Ball Object))
  (Default|IncrementHealth _asbp_ball (Variables|Default|GetHealth))
  (Default|IncrementGoal _asbp_ball)
  (Default|IncrementScore _asbp_ball (Variables|Default|GetPoints))
  (Audio|PlaySound2D (Variables|Default|GetPickupSound) 1.0 1.0 0.0 0 0)
  (Effects|SpawnEmitteratLocation (Variables|Default|GetPickupEmitter) (Transformation|GetActorLocation))
  (if (Variables|Default|GetPickupable?)
    (Rendering|SetVisibility (Variables|Default|GetWidget) true false)
    (Rendering|SetVisibility (Variables|Default|GetStaticMesh) false false)
    (bind _aswbp_pickup_coin (Utilities|Casting|CastToWBP_PickupCoin (UserInterface|GetUserWidgetObject (Variables|Default|GetWidget))))
    (UserInterface|Animation|PlayAnimation _aswbp_pickup_coin (Variables|/Game/Rolling/Blueprints/HUD/WBP_PickupCoin.WBP_PickupCoin_C|GetPickupAnimation _aswbp_pickup_coin) 0.0 1 "Forward" 1.0 false)
    (else
      (Actor|DestroyActor))))