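; BP_Bomb is a pickup variant that acts as an explosive hazard for the rolling ball.
; On pickup it applies a radial velocity impulse to BP_Ball's mesh from just above the bomb, then runs the parent pickup logic.
; At BeginPlay it clears Pickupable, sets an explosion sound and binds to the player ball's DestroyBombs dispatcher.
; When that fires, the bomb plays explosion sound and particles, then destroys itself after a short delay.
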(event Custom|DestroyBombsEvent
  (Audio|PlaySound2D "/Game/StarterContent/Audio/Explosion01.Explosion01" 1.0 1.0 0.0 0 0)
  (Effects|SpawnEmitteratLocation "/Game/InfinityBladeEffects/Effects/FX_Monsters/FX_Monster_Gruntling/Bomber/P_BomberExplode.P_BomberExplode" (Transformation|GetActorLocation))
  (Utilities|FlowControl|Delay 0.2)
  (Actor|DestroyActor))

(event EventBeginPlay
  (Variables|Default|SetPickupable? false)
  (Variables|Default|SetPickupSound "/Game/StarterContent/Audio/Explosion01.Explosion01")
  (|CallParentFunction)
  (bind _asbp_ball (Utilities|Casting|CastToBP_Ball (Game|Player|GetPlayerPawn 0)))
  (EventDispatchers|AssignDestroyBombs _asbp_ball (delegate Custom|DestroyBombsEvent)))

(event EventPickupFunction
  (params (Object :type Object%20Object%20Reference))
  (bind _returnvalue (Transformation|GetActorLocation))
  (bind (_x _y _z) (Math|Vector|BreakVector _returnvalue))
  (bind _asbp_ball (Utilities|Casting|CastToBP_Ball Object))
  (Physics|AddRadialImpulse (Variables|/Game/Rolling/Character/BP_Ball.BP_Ball_C|GetStaticMesh _asbp_ball) (Math|Vector|MakeVector _x _y (+ _z 5e+01)) 3.5e+02 1.5e+03 "RIF_Constant" true)
  (|CallParentFunction Object))

(fn ConstructionScript
  (|CallParentFunction))