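; BP_Fence is a fence actor that builds a straight run of repeated fence meshes from its origin toward an EndPoint offset.
; The construction script divides the EndPoint length by Width to get the segment count, then adds mesh components spaced along local X under the base FenceMeshComponent.
; It then yaws the base component toward EndPoint, turning the attached run with it.
; The event graph holds no active logic.
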(event EventBeginPlay)

(event Collision|EventActorBeginOverlap
  (params (OtherActor :type Actor%20Object%20Reference)))

(event EventTick
  (params (DeltaSeconds :type Float%20%28single-precision%29)))

(fn ConstructionScript
  (bind _returnvalue (Transformation|GetActorLocation))
  (bind _endpoint (Variables|Default|GetEndPoint))
  (bind _width (Variables|Default|Getwidth))
  (bind _returnvalue_2 (Math|Vector|VectorLength _endpoint))
  (bind _returnvalue_3 (/ _returnvalue_2 _width))
  (bind _returnvalue_4 (- _returnvalue_3 1.0))
  (bind _returnvalue_5 (Math|Float|Round _returnvalue_4))
  (Components|StaticMesh|SetStaticMesh (Variables|Default|GetFenceMeshComponent) (Variables|Default|GetFenceMesh))
  (if (>= _returnvalue_5 0)
    (for _index (range 1 _returnvalue_5)
      (bind _returnvalue_6 (AddComponent|AddStaticMeshComponent false))
      (Transformation|AttachComponentToComponent _returnvalue_6 (Variables|Default|GetFenceMeshComponent) "None" "KeepRelative" "KeepRelative" "KeepRelative" true)
      (Transformation|SetRelativeLocation _returnvalue_6 (Math|Vector|MakeVector (* _index (Variables|Default|Getwidth)) 0.0 0.0) false false)
      (Components|StaticMesh|SetStaticMesh _returnvalue_6 (Variables|Default|GetFenceMesh)))
    (Transformation|AddWorldRotation (Variables|Default|GetFenceMeshComponent) (Math|Rotator|MakeRotator 0.0 0.0 (.yaw (Math|Rotator|FindLookatRotation _returnvalue (+ _returnvalue (Variables|Default|GetEndPoint))))) false false)))