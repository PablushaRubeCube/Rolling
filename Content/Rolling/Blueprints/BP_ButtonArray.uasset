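; Pressable floor button for the rolling-ball game that, when a BP_Ball overlaps it, plays a sound, turns red and moves along Z via a timeline.
; On press it calls ButtonMoveReverce on the buttons in ActorArray, restoring their orange color and reversing their movement, like a linked radio-button group.
; The construction script gives each button its own dynamic material instance for the color changes.
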(event OnComponentBeginOverlap(CollisionButton)
  (params (OverlappedComponent :type Primitive%20Component%20Object%20Reference) (OtherActor :type Actor%20Object%20Reference) (OtherComp :type Primitive%20Component%20Object%20Reference) (OtherBodyIndex :type Integer) (bFromSweep :type Boolean) (SweepResult :type Hit%20Result%20Structure%20%28by%20ref%29))
  (bind _initialbuttonlocation (Variables|Default|GetInitialButtonLocation))
  (Utilities|Casting|CastToBP_Ball OtherActor)
  (Audio|PlaySound2D "/Game/Retro_8Bit_Sounds/Collectables/Cues/retro_collect_pickup_item_08_Cue.retro_collect_pickup_item_08_Cue" 1.0 1.0 0.0 0 0)
  (Rendering|Material|SetVectorParameterValue (Variables|Default|GetButtonMaterialInst) "Color" "(R=0.869792,G=0.000000,B=0.000000,A=1.000000)" :!class /Script/Engine.MaterialInstanceDynamic)
  (for _array_element (Variables|Default|GetActorArray)
    (bind _asbp_button_array (Utilities|Casting|CastToBP_ButtonArray _array_element))
    (Default|ButtonMoveReverce _asbp_button_array))
  (bind _buttonmove (Timeline|ButtonDown Play)
    (:Update
      (Transformation|SetWorldLocation (Variables|Default|GetButton) (Math|Vector|MakeVector (.x _initialbuttonlocation) (.y _initialbuttonlocation) (+ _buttonmove (.z _initialbuttonlocation))) false false))))

(event EventBeginPlay
  (Variables|Default|SetInitialButtonLocation (Transformation|GetWorldLocation (Variables|Default|GetButton))))

(event EventButtonMoveReverce
  (bind _initialbuttonlocation (Variables|Default|GetInitialButtonLocation))
  (Rendering|Material|SetVectorParameterValue (Variables|Default|GetButtonMaterialInst) "Color" "(R=0.800000,G=0.300000,B=0.000000,A=1.000000)" :!class /Script/Engine.MaterialInstanceDynamic)
  (bind _buttonmove (Timeline|ButtonDown Reverse)
    (:Update
      (Transformation|SetWorldLocation (Variables|Default|GetButton) (Math|Vector|MakeVector (.x _initialbuttonlocation) (.y _initialbuttonlocation) (+ _buttonmove (.z _initialbuttonlocation))) false false))))

(fn ConstructionScript
  (bind _returnvalue (Rendering|Material|CreateDynamicMaterialInstance "/Game/Rolling/Materials/ButtonMaterialInstance.ButtonMaterialInstance" "None" "None" :!class /Script/Engine.KismetMaterialLibrary))
  (bind _output_get (Variables|Default|SetButtonMaterialInst _returnvalue))
  (Rendering|Material|SetMaterial (Variables|Default|GetButton) 0 _output_get))